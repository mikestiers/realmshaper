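; BP_Pawn is a player camera pawn with smoothed planar movement and spring-arm zoom.
; Forward and Right axis inputs offset a desired location along the actor's forward and right vectors, while Zoom input adjusts a desired arm length clamped between limits.
; Tick eases the actor location and SpringArm length toward those targets with VInterpTo and FInterpTo, moving without sweep collision.
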(event `self.ReceiveBeginPlay`
  (set `self.LocationDesired` (`self.K2_GetActorLocation`))
  (set `self.ZoomDesired` (`SpringArmComponent.TargetArmLength` (`self.SpringArm`))))

(event `self.ReceiveTick`
  (params (DeltaSeconds :type "Float (single-precision)"))
  (bind _springarm (`self.SpringArm`))
  ;[1 1 1] Camera Zoom
  (set `SpringArmComponent.TargetArmLength` (`KismetMathLibrary.FInterpTo` (`SpringArmComponent.TargetArmLength` _springarm) (`self.ZoomDesired`) DeltaSeconds (`self.ZoomInterpSpeed`)) _springarm)
  ;[1 1 1] Camera Movement
  (`self.K2_SetActorLocation` (`KismetMathLibrary.VInterpTo` (`self.K2_GetActorLocation`) (`self.LocationDesired`) DeltaSeconds (`self.MovementInterpSpeed`))))

(event `InputAxis|InputAxis_Forward`
  (params (AxisValue :type "Float (single-precision)"))
  (set `self.LocationDesired` (+ (`self.LocationDesired`) (* (`self.GetActorForwardVector`) (* AxisValue (`self.MovementMultiplierSpeed`))))))

(event `InputAxis|InputAxis_Right`
  (params (AxisValue :type "Float (single-precision)"))
  (set `self.LocationDesired` (+ (`self.LocationDesired`) (* (`self.GetActorRightVector`) (* AxisValue (`self.MovementMultiplierSpeed`))))))

(event `InputAxis|InputAxis_Zoom`
  (params (AxisValue :type "Float (single-precision)"))
  (set `self.ZoomDesired` (`KismetMathLibrary.FClamp` (+ (`self.ZoomDesired`) (* (`self.ZoomMultiplierSpeed`) AxisValue)) (`self.CameraZoomMin`) (`self.CameraZoomMax`))))

(fn `UserConstructionScript`)