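; BP_GridVisual renders the tile grid through two child BP_GridMeshInstance actors: a flat view and a tactical 3D view.
; Tile updates re-add instances, with the flat layer showing only walkable tiles at a ground offset.
; Tactical tiles are colored by type and stretched in Z down to the grid's lowest point, rebuilding lazily when tactical mode is enabled.
; Toggling tactical mode also hides actors tagged NotTactical.
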(event `self.ReceiveBeginPlay`
  (`self.SetActorTickEnabled` false))

(fn `DestroyGridVisual`
  (bind _gridmeshinstance (`self.GridMeshInstance`))
  (bind _gridmeshinstancetactical (`self.GridMeshInstanceTactical`))
  (`|ExecutionSequence`
    (:`then_0`
      (`/Engine/EditorBlueprintResources/StandardMacros.IsValid` _gridmeshinstance
        (:`Is Valid`
          (`/Game/Blueprints/Core/Grid/Utilities/BP_GridMeshInstance.ClearInstances` _gridmeshinstance))))
    (:`then_1`
      (`/Engine/EditorBlueprintResources/StandardMacros.IsValid` _gridmeshinstancetactical
        (:`Is Valid`
          (`/Game/Blueprints/Core/Grid/Utilities/BP_GridMeshInstance.ClearInstances` _gridmeshinstancetactical))))
    (:`then_2`
      (`self.SetGridLowestZ` 999999.0))))

(fn `InitializeGridVisual`
  (params (Grid :type "/Game/Blueprints/Core/Grid/BP_Grid Object Reference"))
  (bind (_meshsize _mesh _meshmaterial) (break `/Game/Blueprints/Core/Grid/GridShapes/S_GridShapeData` (`/Game/Blueprints/Core/Grid/BP_Grid.GetCurrentShapeData` (`self.Grid`))))
  (bind (_meshsize_2 _mesh_2 _meshmaterial_2 _flatmesh _flatmaterial) (break `/Game/Blueprints/Core/Grid/GridShapes/S_GridShapeData` (`/Game/Blueprints/Core/Grid/BP_Grid.GetCurrentShapeData` (`self.Grid`))))
  (set `self.Grid` Grid)
  (set `self.GridMeshInstance` (cast `/Game/Blueprints/Core/Grid/Utilities/BP_GridMeshInstance` (`ChildActorComponent.ChildActor` (`self.ChildActor_GridMeshInst`)) :!pure true))
  (set `self.GridMeshInstanceTactical` (cast `/Game/Blueprints/Core/Grid/Utilities/BP_GridMeshInstance` (`ChildActorComponent.ChildActor` (`self.ChildActor_GridMeshInst_Tactical`)) :!pure true))
  (`/Game/Blueprints/Core/Grid/Utilities/BP_GridMeshInstance.InitializeGridMeshInst` (`self.GridMeshInstance`) _flatmesh _flatmaterial false "QueryOnly")
  (`/Game/Blueprints/Core/Grid/Utilities/BP_GridMeshInstance.InitializeGridMeshInst` (`self.GridMeshInstanceTactical`) _mesh _meshmaterial true "QueryOnly")
  (`self.K2_SetActorLocation` (0.0 0.0 0.0))
  (`self.SetOffsetFromGround` (`self.OffsetFromGround`))
  (`self.SetGridLowestZ` 999999.0)
  (`self.SetIsTactical` (`self.IsTactical`)))

(fn `SetGridLowestZ`
  (params (GridLowestZ :type "Float (double-precision)" :default 999999.0))
  (set `self.GridLowestZ` GridLowestZ)
  (set `self.NeedToRegenerateTacticalOnNextEnable` true))

(fn `SetIsTactical`
  (params (Tactical :type Boolean))
  (set `self.IsTactical` Tactical)
  (`SceneComponent.SetHiddenInGame` (`self.ChildActor_GridMeshInst_Tactical`) (not (`self.IsTactical`)) false)
  (bind _outactors (`GameplayStatics.GetAllActorsWithTag` "NotTactical"))
  (for _array_element _outactors
    (`self.SetActorHiddenInGame` _array_element (`self.IsTactical`)))
  (if (and (`self.IsTactical`) (`self.NeedToRegenerateTacticalOnNextEnable`))
    (set `self.NeedToRegenerateTacticalOnNextEnable` false)
    (bind _values (`BlueprintMapLibrary.Map_Values` (`/Game/Blueprints/Core/Grid/BP_Grid.GridTiles` (`self.Grid`))))
    (for _array_element_2 _values
      (`self.UpdateTileVisualTactical` _array_element_2))))

(fn `SetOffsetFromGround`
  (params (Offset :type "Float (double-precision)"))
  (set `self.OffsetFromGround` Offset)
  (`SceneComponent.K2_SetRelativeLocation` (`self.ChildActor_GridMeshInst`) (`KismetMathLibrary.MakeVector` 0.0 0.0 (`self.OffsetFromGround`)) false false))

(fn `UpdateTileVisual`
  (params (Data :type "/Game/Blueprints/Core/Grid/Utilities/S_TileData Structure"))
  (bind (_data_index _data_tiletype) (break `/Game/Blueprints/Core/Grid/Utilities/S_TileData` (`local.Data`)))
  (bind (_data_index_2 _data_tiletype_2 _data_transform _data_states) (break `/Game/Blueprints/Core/Grid/Utilities/S_TileData` (`local.Data`)))
  (`|ExecutionSequence`
    (:`then_0`
      (`/Game/Blueprints/Core/Grid/Utilities/BP_GridMeshInstance.RemoveInstance` (`self.GridMeshInstance`) _data_index)
      (if (`/Game/Blueprints/Core/Grid/Utilities/BFL_TileData.Is Tile Type Walkable` _data_tiletype)
        (`/Game/Blueprints/Core/Grid/Utilities/BP_GridMeshInstance.AddInstance` (`self.GridMeshInstance`) _data_index_2 _data_transform _data_tiletype_2 _data_states)))
    (:`then_1`
      (`self.UpdateTileVisualTactical` Data))))

(fn `UpdateTileVisualTactical`
  (params (Data :type "/Game/Blueprints/Core/Grid/Utilities/S_TileData Structure"))
  (bind (_data_index _data_tiletype _data_transform _data_states) (break `/Game/Blueprints/Core/Grid/Utilities/S_TileData` (`local.Data`)))
  (bind (_data_index_2 _data_tiletype_2 _data_transform_2) (break `/Game/Blueprints/Core/Grid/Utilities/S_TileData` (`local.Data`)))
  (bind (_data_index_3 _data_tiletype_3 _data_transform_3) (break `/Game/Blueprints/Core/Grid/Utilities/S_TileData` (`local.Data`)))
  (bind (_data_index_4 _data_tiletype_4) (break `/Game/Blueprints/Core/Grid/Utilities/S_TileData` (`local.Data`)))
  (bind _z (.z (`.MeshSize_3_9BBE073B42ED7034C4BA68A9BB2178EC` (break `/Game/Blueprints/Core/Grid/GridShapes/S_GridShapeData` (`/Game/Blueprints/Core/Grid/BP_Grid.GetCurrentShapeData` (`self.Grid`))))))
  (`|ExecutionSequence`
    (:`then_0`
      (if (< (.z (.location _data_transform_2)) (`self.GridLowestZ`))
        (`self.SetGridLowestZ` (.z (.location _data_transform_2)))))
    (:`then_1`
      (if (`self.IsTactical`)
        (`/Game/Blueprints/Core/Grid/Utilities/BP_GridMeshInstance.RemoveInstance` (`self.GridMeshInstanceTactical`) _data_index_4)
        (if (`|EnumInequality` _data_tiletype_4 "NewEnumerator0")
          (`/Game/Blueprints/Core/Grid/Utilities/BP_GridMeshInstance.AddInstance` (`self.GridMeshInstanceTactical`) _data_index (`KismetMathLibrary.MakeTransform` (.location _data_transform) (.rotation _data_transform) (`KismetMathLibrary.MakeVector` (.x (.scale _data_transform)) (.y (.scale _data_transform)) (/ (+ (- (.z (.location _data_transform_3)) (`self.GridLowestZ`)) _z) _z))) _data_tiletype _data_states))
        (else
          (set `self.NeedToRegenerateTacticalOnNextEnable` true))))))

(fn `UserConstructionScript`)