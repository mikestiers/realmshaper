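; BP_Unit is a unit actor whose appearance is driven by its UnitType, with test logic that cycles through animation states.
; The construction script looks up the default unit data for that type and applies its mesh and animation Blueprint to the skeletal mesh.
; From BeginPlay, a looping delay periodically advances a test index through six states and sends each to the anim instance as a message.
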(event `self.ReceiveBeginPlay`
  (`KismetSystemLibrary.Delay` 3.0 :!label _label)
  (bind _output_get (set `self.TestAnimIndex` (cast `/Game/Art/Units/E_UnitAnimationState` (mod (+ (`self.TestAnimIndex`) 1) 6))))
  (message `/Game/Art/Units/BPI_UnitAnimation.SetUnitAnimationState` (`SkeletalMeshComponent.GetAnimInstance` (`self.SkeletalMesh`)) _output_get)
  (goto _label))

(fn `UserConstructionScript`
  (bind _unitdata (`/Game/Blueprints/Core/Units/Utilities/BFL_Units.GetDefaultUnitDataFromUnitType` (`self.UnitType`)))
  (bind (_mesh _animbp) (break `/Game/Blueprints/Core/Units/Utilities/S_UnitData_Assets` (`.Assets_6_1E10E0D74E09BA2B01407C8DFFA579D9` (break `/Game/Blueprints/Core/Units/Utilities/S_UnitData` _unitdata))))
  (`SkeletalMeshComponent.SetSkeletalMeshAsset` (`self.SkeletalMesh`) _mesh)
  (`SkeletalMeshComponent.SetAnimInstanceClass` (`self.SkeletalMesh`) _animbp))